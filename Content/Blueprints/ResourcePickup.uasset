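; Resource pickup actor that grants the player a randomly sized amount of a named resource, such as a metal or element.
; On BeginPlay it sets its mesh, writes its name to a widget label and rolls the amount.
; When the player first overlaps its box, it disables physics and collision, flies to the player while a timeline scales it.
; When the timeline ends, it adds the amount to the matching game mode counter and destroys itself.
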(event `self.ReceiveBeginPlay`
  (`StaticMeshComponent.SetStaticMesh` (`self.StaticMesh1`) (`self.New Mesh`))
  (bind _asname (cast `/Game/widgets/name` (`WidgetComponent.GetWidget` (`self.name`))))
  (set `/Game/widgets/name.name` (`self.name_0`) _asname)
  (set `self.increment` (`KismetMathLibrary.RandomIntegerInRange` 250 1500)))

(event `self.Box.OnComponentBeginOverlap`
  (params (OverlappedComponent :type "PrimitiveComponent Object Reference") (OtherActor :type "Actor Object Reference") (OtherComp :type "PrimitiveComponent Object Reference") (OtherBodyIndex :type Integer) (bFromSweep :type Boolean) (SweepResult :type "HitResult Structure (by ref)"))
  (bind _increment (`self.increment`))
  (bind _staticmesh1 (`self.StaticMesh1`))
  (bind _asplayer (cast `/Game/Blueprints/Player` OtherActor))
  (set `self.As Player` _asplayer)
  (`/Engine/EditorBlueprintResources/StandardMacros.DoOnce` false
    (:`Completed`
      (`PrimitiveComponent.SetSimulatePhysics` _staticmesh1 false)
      (`PrimitiveComponent.SetCollisionEnabled` _staticmesh1 "NoCollision")
      (`KismetSystemLibrary.MoveComponentTo` (`self.RootComponent`) (`self.K2_GetActorLocation` (`self.As Player`)) (struct) false false 0.75)
      (bind (_direction _1) (`Timeline|Timeline`)
        (:`Update`
          (`self.SetActorScale3D` (`KismetMathLibrary.MakeVector` _1 _1 _1)))
        (:`Finished`
          (bind _asmaingm (cast `/Game/Blueprints/maingm` (`GameplayStatics.GetGameMode`)))
          (switch `string` (`KismetTextLibrary.Conv_TextToString` (`self.name_0`))
            (:`iron`
              (set `/Game/Blueprints/maingm.iron` (+ (`/Game/Blueprints/maingm.iron` _asmaingm) _increment) _asmaingm))
            (:`silver`
              (set `/Game/Blueprints/maingm.silver` (+ (`/Game/Blueprints/maingm.silver` _asmaingm) _increment) _asmaingm))
            (:`gold`
              (set `/Game/Blueprints/maingm.gold` (+ (`/Game/Blueprints/maingm.gold` _asmaingm) _increment) _asmaingm))
            (:`silicon`
              (set `/Game/Blueprints/maingm.silicon` (+ _increment (`/Game/Blueprints/maingm.silicon` _asmaingm)) _asmaingm))
            (:`nitrogen`
              (set `/Game/Blueprints/maingm.nitrogen` (+ _increment (`/Game/Blueprints/maingm.nitrogen` _asmaingm)) _asmaingm))
            (:`hydrogen`
              (set `/Game/Blueprints/maingm.hydrogen` (+ _increment (`/Game/Blueprints/maingm.hydrogen` _asmaingm)) _asmaingm))
            (:`carbon`
              (set `/Game/Blueprints/maingm.carbon` (+ _increment (`/Game/Blueprints/maingm.carbon` _asmaingm)) _asmaingm))
            (:`oxygen`
              (set `/Game/Blueprints/maingm.oxygen` (+ _increment (`/Game/Blueprints/maingm.oxygen` _asmaingm)) _asmaingm)))
          (`self.K2_DestroyActor`))))))

(fn `UserConstructionScript`)