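; BP_FieldSpawner is an environment actor that fills a cubic volume around itself with randomly scattered instances of a configurable class.
; On BeginPlay it spawns Amount actors at random offsets within a Distance-sized box, with uniform scale jittered 20% around Scale and no rotation.
; Spawns adjust position to avoid collisions or are skipped.
; The construction script scales the Area component from Distance, matching it to the spawn extent.
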(event `self.ReceiveBeginPlay`
  (bind _scale (`self.Scale`))
  (bind _returnvalue (/ (`self.Distance`) 2.0))
  (bind _returnvalue_2 (* _returnvalue -1.0))
  (for _ (range 1 (+ (`self.Amount`) 1))
    (`|SpawnActorFromClass` (`self.Class to Spawn`) (`KismetMathLibrary.MakeTransform` (+ (`self.K2_GetActorLocation`) (`KismetMathLibrary.MakeVector` (`KismetMathLibrary.RandomFloatInRange` _returnvalue_2 _returnvalue) (`KismetMathLibrary.RandomFloatInRange` _returnvalue_2 _returnvalue) (`KismetMathLibrary.RandomFloatInRange` _returnvalue_2 _returnvalue))) (struct) (`KismetMathLibrary.Conv_DoubleToVector` (`KismetMathLibrary.RandomFloatInRange` (* _scale 0.8) (* _scale 1.2)))) "AdjustIfPossibleButDontSpawnIfColliding" "OverrideRootScale" null null)))

(fn `UserConstructionScript`
  (bind _returnvalue (/ (`self.Distance`) 100.0))
  (`SceneComponent.SetWorldScale3D` (`self.Area`) (`KismetMathLibrary.MakeVector` _returnvalue _returnvalue _returnvalue)))