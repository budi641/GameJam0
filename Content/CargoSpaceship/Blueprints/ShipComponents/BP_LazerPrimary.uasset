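; BP_LazerPrimary is the primary laser weapon component actor of a cargo spaceship.
; Its Fire event spawns a BP_LazerProjectile at its own location and rotation, then plays a firing sound there.
; The weapon's LazerPrimary variables set the projectile's scale, color, damage, speed, physics forces, explosion and lighting, and it passes ParentShip along as the firing ship.
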(event `Fire`
  (bind _returnvalue (`self.K2_GetActorLocation`))
  (`|SpawnActorFromClass` "/Game/CargoSpaceship/Blueprints/ShipComponents/BP_LazerProjectile.BP_LazerProjectile_C" (`KismetMathLibrary.MakeTransform` _returnvalue (`self.K2_GetActorRotation`) (`KismetMathLibrary.Conv_DoubleToVector` (`self.Lazer_Primary_Scale`))) "Undefined" "OverrideRootScale" null (`self.Lazer_Primary_Color`) (`self.Lazer_Primary_PhysicsForce`) (`self.Lazer_Primary_ExplosionScale`) (`self.ParentShip`) (`self.Lazer_Primary_DamageToApply`) (`self.Lazer_Primary_PhysicsForce_Multiplier_ForShield`) (`self.Lazer_Primary_Speed`) (`self.Lazer_Primary_ExplosionBrightness`) (`self.Lazer_Primary_PointLightBrightness`) (`self.Lazer_Primary_PointLightEnabled`) (`self.Lazer_Primary_MaterialGlowIntensity`) self)
  (`GameplayStatics.PlaySoundAtLocation` (`self.Lazer_Primary_SoundCue`) _returnvalue (struct) 1.0 1.0 0.0 null null null null))

(fn `UserConstructionScript`)