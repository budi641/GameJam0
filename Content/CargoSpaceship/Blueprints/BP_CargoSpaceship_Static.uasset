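; Static cargo spaceship prop with configurable look, thruster rotation, optional container, collision toggle and either an animated or fixed door.
; The construction script rotates the engines, removes unused components, sets the fixed door open or closed, and builds dynamic materials for camo or plain hull, colors and cockpit glow, with thrust glow off.
; In animated mode, trigger overlaps play or reverse a timeline that lifts the door, with a sound on each.
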(event `self.Door_Trigger.OnComponentBeginOverlap`
  (params (OverlappedComponent :type "PrimitiveComponent Object Reference") (OtherActor :type "Actor Object Reference") (OtherComp :type "PrimitiveComponent Object Reference") (OtherBodyIndex :type Integer) (bFromSweep :type Boolean) (SweepResult :type "HitResult Structure (by ref)"))
  (`|ExecutionSequence`
    (:`then_0`
      (`GameplayStatics.PlaySoundAtLocation` "/Game/CargoSpaceship/Sounds/SC_ScifiDoor_A.SC_ScifiDoor_A" (`SceneComponent.K2_GetComponentLocation` (`self.Movable_Door_Animated`)) (struct) 1.0 1.0 0.0 null null null null :!label _label))
    (:`then_1`
      (bind (_direction _door_animation) (`Timeline|Timeline_0` :!label _label_2)
        (:`Update`
          (`SceneComponent.K2_SetRelativeLocation` (`self.Movable_Door_Animated`) (`KismetMathLibrary.MakeVector` 0.0 0.0 (`KismetMathLibrary.Lerp` 0.0 172.0 _door_animation)) false false))))))

(event `self.Door_Trigger.OnComponentEndOverlap`
  (params (OverlappedComponent :type "PrimitiveComponent Object Reference") (OtherActor :type "Actor Object Reference") (OtherComp :type "PrimitiveComponent Object Reference") (OtherBodyIndex :type Integer))
  (`|ExecutionSequence`
    (:`then_0`
      (goto _label))
    (:`then_1`
      (goto _label_2 :!via `Reverse`))))

(fn `UserConstructionScript`
  (bind _sm_cargospaceship_body (`self.SM_CargoSpaceship_Body`))
  (bind _sm_cargospaceship_interior (`self.SM_CargoSpaceship_Interior`))
  (bind _sm_cargospaceship_interiorprops (`self.SM_CargoSpaceship_InteriorProps`))
  (bind _hull_material (`self.Hull_Material`))
  (bind _static_door (`self.Static_Door`))
  (`SceneComponent.K2_AddRelativeRotation` (`self.SM_CargoSpaceship_Engine_R1`) (`KismetMathLibrary.MakeRotator` 0.0 (`self.Thruster_Rotation`)) false false)
  (`SceneComponent.K2_AddRelativeRotation` (`self.SM_CargoSpaceship_Engine_L`) (`KismetMathLibrary.MakeRotator` 0.0 (`self.Thruster_Rotation`)) false false)
  (`SceneComponent.K2_AddRelativeRotation` (`self.SM_CargoSpaceship_Engine_L1`) (`KismetMathLibrary.MakeRotator` 0.0 (`self.Thruster_Rotation`)) false false)
  (`SceneComponent.K2_AddRelativeRotation` (`self.SM_CargoSpaceship_Engine_R`) (`KismetMathLibrary.MakeRotator` 0.0 (`self.Thruster_Rotation`)) false false)
  (if (not (`self.Collision`))
    (`PrimitiveComponent.SetCollisionEnabled` (`self.SM_CargoSpaceship_Body`) "NoCollision")
    (`PrimitiveComponent.SetCollisionEnabled` (`self.SM_CargoSpaceship_Engine_L`) "NoCollision")
    (`PrimitiveComponent.SetCollisionEnabled` (`self.SM_CargoSpaceship_Engine_L1`) "NoCollision")
    (`PrimitiveComponent.SetCollisionEnabled` (`self.SM_CargoSpaceship_Engine_R1`) "NoCollision")
    (`PrimitiveComponent.SetCollisionEnabled` (`self.SM_CargoSpaceship_Engine_R`) "NoCollision")
    (`PrimitiveComponent.SetCollisionEnabled` (`self.SM_CargoSpaceship_Interior`) "NoCollision")
    (`PrimitiveComponent.SetCollisionEnabled` (`self.SM_CargoSpaceship_InteriorProps`) "NoCollision")
    (`PrimitiveComponent.SetCollisionEnabled` (`self.SM_RTS14_CargoSpaceship_Seat`) "NoCollision")
    (`PrimitiveComponent.SetCollisionEnabled` (`self.Static_Door`) "NoCollision")
    (`PrimitiveComponent.SetCollisionEnabled` (`self.SM_RTS14_CargoSpaceship_Container`) "NoCollision"))
  (if (`self.Camouflage`)
    (bind _returnvalue (`PrimitiveComponent.CreateDynamicMaterialInstance` _sm_cargospaceship_body 0 "/Game/CargoSpaceship/Materials/CargoSpaceship/MI_CargoSpaceship_Camo.MI_CargoSpaceship_Camo" "None"))
    (bind _output_get (set `self.Hull_Material` _returnvalue))
    (`PrimitiveComponent.SetMaterial` _sm_cargospaceship_body 0 _output_get)
    (`PrimitiveComponent.SetMaterial` (`self.SM_RTS14_CargoSpaceship_Container`) 0 _output_get)
    (`PrimitiveComponent.SetMaterial` (`self.SM_CargoSpaceship_Engine_R`) 0 _output_get)
    (`PrimitiveComponent.SetMaterial` (`self.SM_CargoSpaceship_Engine_L`) 0 _output_get)
    (`PrimitiveComponent.SetMaterial` (`self.SM_CargoSpaceship_Engine_L1`) 0 _output_get)
    (`PrimitiveComponent.SetMaterial` (`self.SM_CargoSpaceship_Engine_R1`) 0 _output_get)
    (else
      (bind _returnvalue_2 (`PrimitiveComponent.CreateDynamicMaterialInstance` _sm_cargospaceship_body 0 "/Game/CargoSpaceship/Materials/CargoSpaceship/MI_CargoSpaceship_Plain.MI_CargoSpaceship_Plain" "None"))
      (bind _output_get_2 (set `self.Hull_Material` _returnvalue_2))
      (`PrimitiveComponent.SetMaterial` _sm_cargospaceship_body 0 _output_get_2)
      (`PrimitiveComponent.SetMaterial` (`self.SM_RTS14_CargoSpaceship_Container`) 0 _output_get_2)
      (`PrimitiveComponent.SetMaterial` (`self.SM_CargoSpaceship_Engine_R1`) 0 _output_get_2)
      (`PrimitiveComponent.SetMaterial` (`self.SM_CargoSpaceship_Engine_L1`) 0 _output_get_2)
      (`PrimitiveComponent.SetMaterial` (`self.SM_CargoSpaceship_Engine_L`) 0 _output_get_2)
      (`PrimitiveComponent.SetMaterial` (`self.SM_CargoSpaceship_Engine_R`) 0 _output_get_2)))
  (`MaterialInstanceDynamic.SetVectorParameterValue` _hull_material "Dif_Color" (`self.Ship_Color`))
  (`MaterialInstanceDynamic.SetVectorParameterValue` _hull_material "Dif_Container_Color" (`self.Container_Color`))
  (`MaterialInstanceDynamic.SetScalarParameterValue` _hull_material "Metal_Tex_Value_A" (`self.Ship_Metallic`))
  (`MaterialInstanceDynamic.SetScalarParameterValue` _hull_material "Rough_Text_Value_B" (`self.Ship_Roughness`))
  (`MaterialInstanceDynamic.SetScalarParameterValue` _hull_material "Thrust_On?" 0.0)
  (bind _returnvalue_3 (`PrimitiveComponent.CreateDynamicMaterialInstance` _sm_cargospaceship_interior 0 "/Game/CargoSpaceship/Materials/CargoSpaceship/Interior/MI_CargoSpaceship_Int_0.MI_CargoSpaceship_Int_0" "None"))
  (bind _output_get_3 (set `self.Interior_Material_0` _returnvalue_3))
  (`PrimitiveComponent.SetMaterial` _sm_cargospaceship_interior 0 _output_get_3)
  (bind _returnvalue_4 (`PrimitiveComponent.CreateDynamicMaterialInstance` _sm_cargospaceship_interior 1 "/Game/CargoSpaceship/Materials/CargoSpaceship/Interior/MI_CargoSpaceship_Int_1.MI_CargoSpaceship_Int_1" "None"))
  (bind _output_get_4 (set `self.Interior_Material_1` _returnvalue_4))
  (`PrimitiveComponent.SetMaterial` _sm_cargospaceship_interior 1 _output_get_4)
  (bind _returnvalue_5 (`PrimitiveComponent.CreateDynamicMaterialInstance` _sm_cargospaceship_interior 2 "/Game/CargoSpaceship/Materials/CargoSpaceship/Interior/MI_CargoSpaceship_Int_2.MI_CargoSpaceship_Int_2" "None"))
  (bind _output_get_5 (set `self.Interior_Material_2` _returnvalue_5))
  (`PrimitiveComponent.SetMaterial` _sm_cargospaceship_interior 2 _output_get_5)
  (bind _returnvalue_6 (`PrimitiveComponent.CreateDynamicMaterialInstance` _sm_cargospaceship_interior 3 "/Game/CargoSpaceship/Materials/CargoSpaceship/Interior/MI_CargoSpaceship_Int_3.MI_CargoSpaceship_Int_3" "None"))
  (bind _output_get_6 (set `self.Interior_Material_3` _returnvalue_6))
  (`PrimitiveComponent.SetMaterial` _sm_cargospaceship_interior 3 _output_get_6)
  (bind _returnvalue_7 (`PrimitiveComponent.CreateDynamicMaterialInstance` _sm_cargospaceship_interiorprops 0 "/Game/CargoSpaceship/Materials/CargoSpaceship/Interior/MI_CargoSpaceship_Props.MI_CargoSpaceship_Props" "None"))
  (bind _output_get_7 (set `self.InteriorProps_Material` _returnvalue_7))
  (`PrimitiveComponent.SetMaterial` _sm_cargospaceship_interiorprops 0 _output_get_7)
  (`MaterialInstanceDynamic.SetScalarParameterValue` (`self.Hull_Material`) "Glow_Cockpit" (`self.Cockpit_Glow_Amount`))
  (`MaterialInstanceDynamic.SetScalarParameterValue` (`self.Interior_Material_3`) "Glow_Cockpit" (`self.Cockpit_Glow_Amount`))
  (`MaterialInstanceDynamic.SetScalarParameterValue` (`self.Interior_Material_2`) "Glow_Cockpit" (`self.Cockpit_Glow_Amount`))
  (`MaterialInstanceDynamic.SetScalarParameterValue` (`self.Interior_Material_1`) "Glow_Cockpit" (`self.Cockpit_Glow_Amount`))
  (`MaterialInstanceDynamic.SetScalarParameterValue` (`self.Interior_Material_0`) "Glow_Cockpit" (`self.Cockpit_Glow_Amount`))
  (`MaterialInstanceDynamic.SetScalarParameterValue` (`self.InteriorProps_Material`) "Glow_Cockpit" (`self.Cockpit_Glow_Amount`))
  (`MaterialInstanceDynamic.SetScalarParameterValue` (`self.Hull_Material`) "Glow_Cockpit_Highlights" (`self.Cockpit_Glow_Highlights_Amount`))
  (`MaterialInstanceDynamic.SetScalarParameterValue` (`self.Interior_Material_3`) "Glow_Cockpit_Highlights" (`self.Cockpit_Glow_Highlights_Amount`))
  (`MaterialInstanceDynamic.SetScalarParameterValue` (`self.Interior_Material_2`) "Glow_Cockpit_Highlights" (`self.Cockpit_Glow_Highlights_Amount`))
  (`MaterialInstanceDynamic.SetScalarParameterValue` (`self.Interior_Material_1`) "Glow_Cockpit_Highlights" (`self.Cockpit_Glow_Highlights_Amount`))
  (`MaterialInstanceDynamic.SetScalarParameterValue` (`self.Interior_Material_0`) "Glow_Cockpit_Highlights" (`self.Cockpit_Glow_Highlights_Amount`))
  (`MaterialInstanceDynamic.SetScalarParameterValue` (`self.InteriorProps_Material`) "Glow_Cockpit_Highlights" (`self.Cockpit_Glow_Highlights_Amount`))
  (if (not (`self.Include Container?`))
    (`ActorComponent.K2_DestroyComponent` (`self.SM_RTS14_CargoSpaceship_Container`)))
  ;[1 1 1] Door
  (if (`self.Animated_Door?`)
    (`ActorComponent.K2_DestroyComponent` (`self.Static_Door`))
    (else
      (`ActorComponent.K2_DestroyComponent` (`self.Movable_Door_Animated`))
      (if (`self.Door_Open?`)
        (`SceneComponent.K2_SetRelativeLocation` _static_door (704.099976 0.0 450.0) false false)
        (else
          (`SceneComponent.K2_SetRelativeLocation` _static_door (704.099976 0.0 278.700012) false false))))))